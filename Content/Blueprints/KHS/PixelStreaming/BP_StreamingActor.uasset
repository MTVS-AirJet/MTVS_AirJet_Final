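; Actor that receives Pixel Streaming video in-game by acting as a WebRTC client to a remote signalling server.
; On BeginPlay it connects to a hardcoded WebSocket address and subscribes to the first available streamer.
; Signalling and peer components relay config, offer/answer and ICE candidates to each other.
; Functions subscribe to a given streamer ID, switch streams, or unsubscribe and disconnect.
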(event OnConnected(PixelStreamingSignalling)
  (bind _streamerlist (|GetStreamerIdList (Variables|Default|GetPixelStreamingSignalling))
    (:Completed
      (if (> (Utilities|Array|Length _streamerlist) 0)
        (Class|PixelStreamingSignallingComponent|Subscribe (Variables|Default|GetPixelStreamingSignalling) (Utilities|Array|Get(acopy) _streamerlist))))))

(event OnConfig(PixelStreamingSignalling)
  (params (Config :type Pixel%20Streaming%20RTC%20Config%20Wrapper%20Structure))
  (Class|PixelStreamingPeerComponent|SetConfig (Variables|Default|GetPixelStreamingPeer) Config))

(event OnOffer(PixelStreamingSignalling)
  (params (Offer :type String))
  (bind _returnvalue (Class|PixelStreamingPeerComponent|CreateAnswer (Variables|Default|GetPixelStreamingPeer) Offer))
  (Class|PixelStreamingSignallingComponent|SendAnswer (Variables|Default|GetPixelStreamingSignalling) _returnvalue))

(event OnIceCandidate(PixelStreamingSignalling)
  (params (Candidate :type Pixel%20Streaming%20Ice%20Candidate%20Wrapper%20Structure))
  (Class|PixelStreamingPeerComponent|ReceiveIceCandidate (Variables|Default|GetPixelStreamingPeer) Candidate))

(event OnIceCandidate(PixelStreamingPeer)
  (params (Candidate :type Pixel%20Streaming%20Ice%20Candidate%20Wrapper%20Structure))
  (Class|PixelStreamingSignallingComponent|SendIceCandidate (Variables|Default|GetPixelStreamingSignalling) Candidate))

(event EventBeginPlay
  (Class|PixelStreamingSignallingComponent|Connect (Variables|Default|GetPixelStreamingSignalling) "ws://125.132.216.190:7756"))

(event Collision|EventActorBeginOverlap
  (params (OtherActor :type Actor%20Object%20Reference)))

(event EventTick
  (params (DeltaSeconds :type Float%20%28single-precision%29)))

(fn ConstructionScript)

(fn ChangePixelStreaming
  (params (userID :type String))
  (bind _pixelstreamingsignalling (Variables|Default|GetPixelStreamingSignalling))
  (Class|PixelStreamingSignallingComponent|Unsubscribe _pixelstreamingsignalling)
  (Class|PixelStreamingSignallingComponent|Subscribe _pixelstreamingsignalling userID))

(fn BeginLookPixelStreaming
  (params (ID :type String))
  (Class|PixelStreamingSignallingComponent|Subscribe (Variables|Default|GetPixelStreamingSignalling) ID))

(fn StopLookPixelStreaming
  (bind _pixelstreamingsignalling (Variables|Default|GetPixelStreamingSignalling))
  (Class|PixelStreamingSignallingComponent|Unsubscribe _pixelstreamingsignalling)
  (Class|PixelStreamingSignallingComponent|Disconnect _pixelstreamingsignalling))