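; Trigger box that teleports overlapping BP_Viper jets to a geographic destination in the Cesium world.
; On overlap it moves the georeference origin to the destination coordinates, converts that to Unreal space, places the Viper there at a random height, enables its jet-tail VFX and calls NotifyFlight.
; Once the teleport count matches the Vipers counted at BeginPlay, the Cesium manager moves there too.
; Polygon-overlay relocation and inversion logic is unused.
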(event OnComponentBeginOverlap(BoxComp)
  (params (OverlappedComponent :type Primitive%20Component%20Object%20Reference) (OtherActor :type Actor%20Object%20Reference) (OtherComp :type Primitive%20Component%20Object%20Reference) (OtherBodyIndex :type Integer) (bFromSweep :type Boolean) (SweepResult :type Hit%20Result%20Structure%20%28by%20ref%29)))

(event Custom|SetInvertSelectionTrue
  ;[1 1 1] polygon teleport -> invert selection set
  (bind _outactors (Actor|GetAllActorsOfClasswithTag "/Script/CesiumRuntime.Cesium3DTileset" "3DTile"))
  (Variables|/Script/CesiumRuntime.CesiumPolygonRasterOverlay|SetInvertSelection (Actor|GetComponentbyClass (Utilities|Array|Get(acopy) _outactors) "/Script/CesiumRuntime.CesiumPolygonRasterOverlay") true))

(event EventBeginPlay
  ;[1 1 1] Get Viper Cnt
  (bind _outactors (Actor|GetAllActorsOfClasswithTag "/Game/Blueprints/LHJ/BP_Viper.BP_Viper_C" "Viper"))
  (Variables|Default|SetViperCnt (Utilities|Array|Length _outactors)))

(event Collision|EventActorBeginOverlap
  (params (OtherActor :type Actor%20Object%20Reference))
  ;[1 1 1] Set Destination Location with Longitude/Latitude
  (bind _returnvalue (Class|CesiumGeoreference|GetDefaultGeoreference))
  (Variables|Default|SetCurGeoReference _returnvalue)
  (Class|CesiumGeoreference|SetOriginLongitudeLatitudeHeight _returnvalue (Math|Vector|MakeVector (Variables|Default|GetDestLatitude) (Variables|Default|GetDestLongitude) 0.0))
  (Variables|Default|SetDestLocation (Class|CesiumGeoreference|TransformLongitudeLatitudeHeightPositiontoUnreal (Variables|Default|GetCurGeoReference) (Class|CesiumGeoreference|GetOriginLongitudeLatitudeHeight (Variables|Default|GetCurGeoReference))))
  ;[1 1 1] Teleport Viper
  (bind _asbp_viper (Utilities|Casting|CastToBP_Viper OtherActor))
  (Transformation|SetActorLocation _asbp_viper (Math|Vector|MakeVector (.X (Math|Vector|BreakVector (Variables|Default|GetDestLocation))) (.Y (Math|Vector|BreakVector (Variables|Default|GetDestLocation))) (Math|Random|RandomFloatinRange (.Z (Math|Vector|BreakVector (Variables|Default|GetDestLocation))) 5e+03)) false true)
  (Variables|/Script/MTVS_AirJet_Final.L_Viper|SetbJetTailVFXOn _asbp_viper true)
  (Variables|Default|SetViperTeleportedCnt (+ (Variables|Default|GetViperTeleportedCnt) 1))
  (Networking|SwitchHasAuthority
    (:Authority
      _)
    (:Remote
      _))
  ;[1 1 1] JBS 추가 플레이어 컨트롤러에게 이륙 했음을 알리는 함수
  (Class|KCesiumTeleportBox|NotifyFlight _asbp_viper)
  (if (== (Variables|Default|GetViperCnt) (Variables|Default|GetViperTeleportedCnt))
    ;[1 1 1] Cesium Manager Teleport
    (bind _outactors (Actor|GetAllActorsOfClasswithTag "/Game/Blueprints/KHS/Server/BP_K_CesiumManager.BP_K_CesiumManager_C" "CesiumManager"))
    (Transformation|SetActorLocation (Utilities|Array|Get(acopy) _outactors) (Math|Vector|MakeVector (.x (Variables|Default|GetDestLocation)) (.y (Variables|Default|GetDestLocation)) (.z (Variables|Default|GetDestLocation))) false false)))

(event EventTick
  (params (DeltaSeconds :type Float%20%28single-precision%29)))

(fn ConstructionScript)