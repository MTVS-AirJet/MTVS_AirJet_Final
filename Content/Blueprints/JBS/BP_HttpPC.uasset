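; BP_HttpPC is a debug-input Blueprint, apparently a player controller, that plays voice sounds held by BP_JsonManager one after another.
; BeginPlay adds the IMC_DebugInput mapping context and caches the BP_JsonManager found in the level.
; Each IA_Debug01 press plays the next VoiceAry entry on the Audio component, prints its index in Korean and increments the counter, with no bounds check or wraparound.
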(event Input|EnhancedActionEvents|EnhancedInputActionIA_Debug01
  (params (ActionValue :type Boolean) (ElapsedSeconds :type Float%20%28double-precision%29) (TriggeredSeconds :type Float%20%28double-precision%29) (InputAction :type Input%20Action%20Object%20Reference :default "/Game/Input/JBS/IA_Debug01.IA_Debug01"))
  (bind _voicecnt (Variables|Default|GetvoiceCnt))
  (bind _audio (Variables|Default|GetAudio))
  (:Started
    (Audio|Components|Audio|SetSound _audio (Utilities|Array|Get(acopy) (Variables|/Script/MTVS_AirJet_Final.J_JsonManager|GetvoiceAry (Variables|Default|GetJsonManager)) _voicecnt))
    (Audio|Components|Audio|Play _audio 0.0)
    (Development|PrintString (Utilities|String|Append (Utilities|String|ToString(Integer) _voicecnt) "번째 사운드 재생"))
    (Math|Integer|IncrementInt _voicecnt)))

(event EventBeginPlay
  (Input|AddMappingContext (PlayerController|LocalPlayerSubsystems|GetEnhancedInputLocalPlayerSubsystem) "/Game/Input/JBS/IMC_DebugInput.IMC_DebugInput" 0 "(bIgnoreAllPressedKeysUntilRelease=True,bForceImmediately=False,bNotifyUserSettings=False)")
  (bind _returnvalue (Actor|GetActorOfClass "/Game/Blueprints/JBS/BP_JsonManager.BP_JsonManager_C"))
  (bind _asbp_json_manager (Utilities|Casting|CastToBP_JsonManager _returnvalue))
  (Variables|Default|SetJsonManager _asbp_json_manager))

(event EventTick
  (params (DeltaSeconds :type Float%20%28single-precision%29)))

(fn ConstructionScript)