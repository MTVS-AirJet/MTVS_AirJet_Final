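; BP_J_StreamingActor is a Pixel Streaming receiver actor for viewing shared screens.
; On BeginPlay it connects to the signalling server and, once connected, subscribes to the first listed streamer.
; The signalling and peer components exchange config, offer/answer and ICE candidates to negotiate the WebRTC connection.
; Custom events begin viewing or switch the subscription by UserID, and stopping both unsubscribes and disconnects from the server.
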(event OnConnected(PixelStreamingSignalling)
  (bind _streamerlist (|GetStreamerIdList (Variables|Default|GetPixelStreamingSignalling))
    (:Completed
      (if (> (Utilities|Array|Length _streamerlist) 0)
        (Class|PixelStreamingSignallingComponent|Subscribe (Variables|Default|GetPixelStreamingSignalling) (Utilities|Array|Get(acopy) _streamerlist))))))

(event OnConfig(PixelStreamingSignalling)
  (params (Config :type Pixel%20Streaming%20RTC%20Config%20Wrapper%20Structure))
  (Class|PixelStreamingPeerComponent|SetConfig (Variables|Default|GetPixelStreamingPeer) Config))

(event OnOffer(PixelStreamingSignalling)
  (params (Offer :type String))
  (bind _returnvalue (Class|PixelStreamingPeerComponent|CreateAnswer (Variables|Default|GetPixelStreamingPeer) Offer))
  (Class|PixelStreamingSignallingComponent|SendAnswer (Variables|Default|GetPixelStreamingSignalling) _returnvalue))

(event OnIceCandidate(PixelStreamingSignalling)
  (params (Candidate :type Pixel%20Streaming%20Ice%20Candidate%20Wrapper%20Structure))
  (Class|PixelStreamingPeerComponent|ReceiveIceCandidate (Variables|Default|GetPixelStreamingPeer) Candidate))

(event OnIceCandidate(PixelStreamingPeer)
  (params (Candidate :type Pixel%20Streaming%20Ice%20Candidate%20Wrapper%20Structure))
  (Class|PixelStreamingSignallingComponent|SendIceCandidate (Variables|Default|GetPixelStreamingSignalling) Candidate))

(event EventBeginPlay
  (Class|PixelStreamingSignallingComponent|Connect (Variables|Default|GetPixelStreamingSignalling) (Variables|Default|GetpsServerURL)))

(event EventTick
  (params (DeltaSeconds :type Float%20%28single-precision%29)))

(event EventChangeLookSharingScreen
  (bind _pixelstreamingsignalling (Variables|Default|GetPixelStreamingSignalling))
  ;[1 1 1] 화면 공유 시점 변경
  (Class|PixelStreamingSignallingComponent|Unsubscribe _pixelstreamingsignalling)
  (Class|PixelStreamingSignallingComponent|Subscribe _pixelstreamingsignalling (Variables|Default|GetUserID)))

(event EventBeginLookSharingScreen
  (Class|PixelStreamingSignallingComponent|Subscribe (Variables|Default|GetPixelStreamingSignalling) (Variables|Default|GetUserID)))

(event EventStopLookSharingScreen
  (bind _pixelstreamingsignalling (Variables|Default|GetPixelStreamingSignalling))
  (Class|PixelStreamingSignallingComponent|Unsubscribe _pixelstreamingsignalling)
  (Class|PixelStreamingSignallingComponent|Disconnect _pixelstreamingsignalling))

(fn ConstructionScript)