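; BP_Roler is a temporary actor, kept in a Temp folder, that lets the player pick a role before entering the mission.
; It enables input from the first player controller on BeginPlay.
; Left click sets PlayerRole to Commander and right click to Pilot on BP_K_GameInstance, so the choice persists across the level change.
; Both clicks then share a short delay before opening MissionLevel.
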(event EventBeginPlay
  (Input|EnableInput (Game|GetPlayerController 0)))

(event Collision|EventActorBeginOverlap
  (params (OtherActor :type Actor%20Object%20Reference)))

(event EventTick
  (params (DeltaSeconds :type Float%20%28single-precision%29)))

(event Input|MouseEvents|LeftMouseButton
  (params (Key :type Key%20Structure :default "None"))
  (:Pressed
    (bind _asbp_k_game_instance (Utilities|Casting|CastToBP_K_GameInstance (Game|GetGameInstance)))
    (Variables|/Script/MTVS_AirJet_Final.K_GameInstance|SetplayerRole _asbp_k_game_instance "COMMANDER")
    (Utilities|FlowControl|Delay 1.0)
    (Game|OpenLevel(byObjectReference) "/Game/Maps/JBS/MissionLevel.MissionLevel")))

(event Input|MouseEvents|RightMouseButton
  (params (Key :type Key%20Structure :default "None"))
  (:Pressed
    (bind _asbp_k_game_instance (Utilities|Casting|CastToBP_K_GameInstance (Game|GetGameInstance)))
    (Variables|/Script/MTVS_AirJet_Final.K_GameInstance|SetplayerRole _asbp_k_game_instance "PILOT")
    (Utilities|FlowControl|Delay 1.0)
    (Game|OpenLevel(byObjectReference) "/Game/Maps/JBS/MissionLevel.MissionLevel")))

(fn ConstructionScript)