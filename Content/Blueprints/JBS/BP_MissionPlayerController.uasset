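; BP_MissionPlayerController is the mission player controller, here carrying debug shortcuts for mission flow.
; With debug input enabled, the local controller adds IMC_DebugInput on BeginPlay; Tick prints player 0's pawn name.
; Debug keys register every controller as flighted, complete the active mission or its neutralize-target sub-objective, and show the result UI.
; These act on the server through authority switches or GameMode casts; one disconnected flight-registration branch never runs.
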(event Input|EnhancedActionEvents|EnhancedInputActionIA_Debug02
  (params (ActionValue :type Boolean) (ElapsedSeconds :type Float%20%28double-precision%29) (TriggeredSeconds :type Float%20%28double-precision%29) (InputAction :type Input%20Action%20Object%20Reference :default "/Game/Input/JBS/IA_Debug02.IA_Debug02"))
  (:Started
    ;[1 1 1] 현재 전술 명령 하나 성공 처리
    (Networking|SwitchHasAuthority
      (:Authority
        (bind _asbp_mission_gamemode (Utilities|Casting|CastToBP_MissionGamemode (Game|GetGameMode)))
        (Class|JBaseMissionObjective|ObjectiveEnd (Variables|/Script/MTVS_AirJet_Final.J_ObjectiveManagerComponent|GetcurActiveMission (Variables|/Script/MTVS_AirJet_Final.J_MissionGamemode|GetobjectiveManagerComp _asbp_mission_gamemode)) true)))))

(event Input|EnhancedActionEvents|EnhancedInputActionIA_Debug03
  (params (ActionValue :type Boolean) (ElapsedSeconds :type Float%20%28double-precision%29) (TriggeredSeconds :type Float%20%28double-precision%29) (InputAction :type Input%20Action%20Object%20Reference :default "/Game/Input/JBS/IA_Debug03.IA_Debug03"))
  ;[1 1 1] 현재 결산 화면 스위치
  (:Started
    (Networking|SwitchHasAuthority
      (:Authority
        (Class|JObjectiveUI|ActiveResultUI (Variables|/Script/MTVS_AirJet_Final.J_ObjectiveUIComp|GetobjUI (Variables|Default|GetBP_ObjUIComp)) (Variables|Default|GetResult%20Obj%20Data))))))

(event Input|EnhancedActionEvents|EnhancedInputActionIA_Debug04
  (params (ActionValue :type Boolean) (ElapsedSeconds :type Float%20%28double-precision%29) (TriggeredSeconds :type Float%20%28double-precision%29) (InputAction :type Input%20Action%20Object%20Reference :default "/Game/Input/JBS/IA_Debug04.IA_Debug04"))
  ;[1 1 1] 공대지 서브 목표 하나 성공 처리
  (:Started
    (Networking|SwitchHasAuthority
      (:Authority
        (bind _asbp_mission_gamemode (Utilities|Casting|CastToBP_MissionGamemode (Game|GetGameMode)))
        (bind _asbp_objective_neutralize_target (Utilities|Casting|CastToBP_ObjectiveNeutralizeTarget (Variables|/Script/MTVS_AirJet_Final.J_ObjectiveManagerComponent|GetcurActiveMission (Variables|/Script/MTVS_AirJet_Final.J_MissionGamemode|GetobjectiveManagerComp _asbp_mission_gamemode))))
        (Utilities|IsValid (Utilities|Array|Get(acopy) (Variables|/Script/MTVS_AirJet_Final.J_ObjectiveNeutralizeTarget|GetsubMPArray _asbp_objective_neutralize_target) (Variables|/Script/MTVS_AirJet_Final.J_ObjectiveNeutralizeTarget|GetcurActiveSubMPIdx _asbp_objective_neutralize_target))
          (:Is%20Valid
            (Class|JBaseMissionObjective|ObjectiveEnd (Utilities|Array|Get(acopy) (Variables|/Script/MTVS_AirJet_Final.J_ObjectiveNeutralizeTarget|GetsubMPArray _asbp_objective_neutralize_target) (Variables|/Script/MTVS_AirJet_Final.J_ObjectiveNeutralizeTarget|GetcurActiveSubMPIdx _asbp_objective_neutralize_target)) true)))))))

(event Input|EnhancedActionEvents|EnhancedInputActionIA_Debug01
  (params (ActionValue :type Boolean) (ElapsedSeconds :type Float%20%28double-precision%29) (TriggeredSeconds :type Float%20%28double-precision%29) (InputAction :type Input%20Action%20Object%20Reference :default "/Game/Input/JBS/IA_Debug01.IA_Debug01"))
  ;[1 1 1] 현재 모든 플레이어 미션 시작 텔포
  (:Started
    (bind _asbp_mission_gamemode (Utilities|Casting|CastToBP_MissionGamemode (Game|GetGameMode)))
    (bind _outactors (Actor|GetAllActorsOfClass "BP_MissionPlayerController_C"))
    (for _array_element _outactors
      (Class|JMissionGamemode|AddFlightedPC _asbp_mission_gamemode _array_element true))))

(event EventBeginPlay
  ;[1 1 1] 디버그용 인풋
  (if (and (Variables|Default|GetenableDebugInput) (Pawn|IsLocalPlayerController))
    (Input|AddMappingContext (PlayerController|LocalPlayerSubsystems|GetEnhancedInputLocalPlayerSubsystem) "/Game/Input/JBS/IMC_DebugInput.IMC_DebugInput" 0 "(bIgnoreAllPressedKeysUntilRelease=True,bForceImmediately=False,bNotifyUserSettings=False)")))

(event EventTick
  (params (DeltaSeconds :type Float%20%28single-precision%29))
  (Development|PrintString (Utilities|GetDisplayName (Game|Player|GetPlayerPawn 0)) true true "(R=0.000000,G=0.660000,B=1.000000,A=1.000000)" 0.0))

(fn ConstructionScript)