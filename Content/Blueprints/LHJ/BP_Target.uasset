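; BP_Target is a target actor that continuously slides back and forth between its starting position and a point 200 units along world +Y.
; BeginPlay caches both endpoints, and Tick linearly interpolates between them using accumulated delta time, so each leg takes about one second.
; A boolean Type selects the direction, flipping after the actor snaps to each endpoint and the timer resets.
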(event EventBeginPlay
  (bind _output_get (Variables|Default|SetInitLoc (Transformation|GetActorLocation)))
  (Variables|Default|SetTargetLoc (+ _output_get "0.000000,200.000000,0.000000")))

(event Collision|EventActorBeginOverlap
  (params (OtherActor :type Actor%20Object%20Reference)))

(event EventTick
  (params (DeltaSeconds :type Float%20%28single-precision%29))
  (if (Variables|Default|GetbType)
    (bind _output_get (Variables|Default|Setalpha (+ DeltaSeconds (Variables|Default|Getalpha))))
    (Transformation|SetActorLocation (Math|Vector|Lerp(Vector) (Variables|Default|GetInitLoc) (Variables|Default|GetTargetLoc) _output_get) false false)
    (if (> (Variables|Default|Getalpha) 1.0)
      (Transformation|SetActorLocation (Variables|Default|GetTargetLoc) false false)
      (Variables|Default|SetbType false)
      (Variables|Default|Setalpha 0.0))
    (else
      (bind _output_get_2 (Variables|Default|Setalpha (+ DeltaSeconds (Variables|Default|Getalpha))))
      (Transformation|SetActorLocation (Math|Vector|Lerp(Vector) (Variables|Default|GetTargetLoc) (Variables|Default|GetInitLoc) _output_get_2) false false)
      (if (> (Variables|Default|Getalpha) 1.0)
        (Transformation|SetActorLocation (Variables|Default|GetInitLoc) false false)
        (Variables|Default|SetbType true)
        (Variables|Default|Setalpha 0.0)))))

(fn ConstructionScript)