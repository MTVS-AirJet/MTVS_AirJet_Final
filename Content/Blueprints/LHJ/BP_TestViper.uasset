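; BP_TestViper is a test player-controlled craft, steered by rotating an Arrow component and driven by physics thrust.
; Enhanced Input move and turn actions add to a ForceUnitVector rotation rate, throttled by ChangeTime, and subtract on release.
; Tick applies that rate to the Arrow within pitch and yaw limits, then pushes the mesh along its forward vector while the toggled engine is on.
; Self-centering and mesh-turning logic is disconnected.
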(event Input|EnhancedActionEvents|EnhancedInputActionIA_ViperEngine
  (params (ActionValue :type Boolean) (ElapsedSeconds :type Float%20%28double-precision%29) (TriggeredSeconds :type Float%20%28double-precision%29) (InputAction :type Input%20Action%20Object%20Reference :default "/Game/Input/LHJ/IA/IA_ViperEngine.IA_ViperEngine"))
  ;[1 1 1] 엔진 컨트롤
  (:Started
    (Utilities|FlowControl|FlipFlop
      (:A
        (Variables|Default|SetIsEngineOn true))
      (:B
        (Variables|Default|SetIsEngineOn false)))))

(event Input|EnhancedActionEvents|EnhancedInputActionIA_ViperMoveUp
  (params (ActionValue :type Vector :default "0, 0, 0") (ElapsedSeconds :type Float%20%28double-precision%29) (TriggeredSeconds :type Float%20%28double-precision%29) (InputAction :type Input%20Action%20Object%20Reference :default "/Game/Input/LHJ/IA/IA_ViperMoveUp.IA_ViperMoveUp"))
  ;[1 1 1] Combine Rotate
  (:Triggered
    (if (> (Variables|Default|GetCurrTime) (Variables|Default|GetChangeTime))
      (Variables|Default|SetCurrTime 0.0)
      (bind _newrot (CallFunction|CombineRotate ActionValue))
      (Variables|Default|SetForceUnitVector _newrot))
    (Variables|Default|SetIsKeyUpPress true))
  (:Completed
    (bind _newrot_2 (CallFunction|CombineRotate (* ActionValue -1.0)))
    (Variables|Default|SetForceUnitVector _newrot_2)
    (Variables|Default|SetIsKeyUpPress false)))

(event Input|EnhancedActionEvents|EnhancedInputActionIA_ViperMoveDown
  (params (ActionValue :type Vector :default "0, 0, 0") (ElapsedSeconds :type Float%20%28double-precision%29) (TriggeredSeconds :type Float%20%28double-precision%29) (InputAction :type Input%20Action%20Object%20Reference :default "/Game/Input/LHJ/IA/IA_ViperMoveDown.IA_ViperMoveDown"))
  ;[1 1 1] Combine Rotate
  (:Triggered
    (if (> (Variables|Default|GetCurrTime) (Variables|Default|GetChangeTime))
      (Variables|Default|SetCurrTime 0.0)
      (bind _newrot (CallFunction|CombineRotate ActionValue))
      (Variables|Default|SetForceUnitVector _newrot))
    (Variables|Default|SetIsKeyDownPress true))
  (:Completed
    (bind _newrot_2 (CallFunction|CombineRotate (* ActionValue -1.0)))
    (Variables|Default|SetForceUnitVector _newrot_2)
    (Variables|Default|SetIsKeyDownPress false)))

(event Input|EnhancedActionEvents|EnhancedInputActionIA_ViperTurnLeft
  (params (ActionValue :type Vector :default "0, 0, 0") (ElapsedSeconds :type Float%20%28double-precision%29) (TriggeredSeconds :type Float%20%28double-precision%29) (InputAction :type Input%20Action%20Object%20Reference :default "/Game/Input/LHJ/IA/IA_ViperTurnLeft.IA_ViperTurnLeft"))
  ;[1 1 1] Combine Rotate
  (:Triggered
    (if (> (Variables|Default|GetCurrTime) (Variables|Default|GetChangeTime))
      (Variables|Default|SetCurrTime 0.0)
      (bind _newrot (CallFunction|CombineRotate ActionValue))
      (Variables|Default|SetForceUnitVector _newrot))
    (Variables|Default|SetIsKeyLeftPress true))
  (:Completed
    (bind _newrot_2 (CallFunction|CombineRotate (* ActionValue -1.0)))
    (Variables|Default|SetForceUnitVector _newrot_2)
    (Variables|Default|SetIsKeyLeftPress false)))

(event Input|EnhancedActionEvents|EnhancedInputActionIA_ViperTurnRight
  (params (ActionValue :type Vector :default "0, 0, 0") (ElapsedSeconds :type Float%20%28double-precision%29) (TriggeredSeconds :type Float%20%28double-precision%29) (InputAction :type Input%20Action%20Object%20Reference :default "/Game/Input/LHJ/IA/IA_ViperTurnRight.IA_ViperTurnRight"))
  ;[1 1 1] Combine Rotate
  (:Triggered
    (if (> (Variables|Default|GetCurrTime) (Variables|Default|GetChangeTime))
      (Variables|Default|SetCurrTime 0.0)
      (bind _newrot (CallFunction|CombineRotate ActionValue))
      (Variables|Default|SetForceUnitVector _newrot))
    (Variables|Default|SetIsKeyRightPress true))
  (:Completed
    (bind _newrot_2 (CallFunction|CombineRotate (* ActionValue -1.0)))
    (Variables|Default|SetForceUnitVector _newrot_2)
    (Variables|Default|SetIsKeyRightPress false)))

(event EventBeginPlay
  ;[1 1 1] Enhanced Input Setting
  (bind _asplayer_controller (Utilities|Casting|CastToPlayerController (Pawn|GetController)))
  (Input|AddMappingContext (PlayerController|LocalPlayerSubsystems|GetEnhancedInputLocalPlayerSubsystem _asplayer_controller) "/Game/Input/LHJ/IMC_Viper.IMC_Viper" 0 "(bIgnoreAllPressedKeysUntilRelease=True,bForceImmediately=False,bNotifyUserSettings=False)"))

(event Collision|EventActorBeginOverlap
  (params (OtherActor :type Actor%20Object%20Reference)))

(event EventTick
  (params (DeltaSeconds :type Float%20%28single-precision%29))
  (bind _arrow (Variables|Default|GetArrow))
  (bind _arrow_2 (Variables|Default|GetArrow))
  (bind _arrow_3 (Variables|Default|GetArrow))
  (bind _arrow_4 (Variables|Default|GetArrow))
  (bind _relativerotation (Variables|/Script/Engine.SceneComponent|GetRelativeRotation _arrow_3))
  (bind _relativerotation_2 (Variables|/Script/Engine.SceneComponent|GetRelativeRotation _arrow))
  (bind _relativerotation_3 (Variables|/Script/Engine.SceneComponent|GetRelativeRotation _arrow_4))
  (bind _returnvalue (> (.yaw _relativerotation_2) 89.0))
  (bind _returnvalue_2 (> (.pitch _relativerotation_2) 85.0))
  (Utilities|FlowControl|Sequence
    (:then_0
      ;[1 1 1] Arrow의 회전값을 변경
      ;;[1 1 1] Y축 회전이 범위 안쪽인지 확인
      (if (or _returnvalue_2 (< (.pitch _relativerotation_2) -85.0))
        (if _returnvalue_2
          (Transformation|SetRelativeRotation _arrow_2 (Math|Rotator|MakeRotator (.roll _relativerotation) 84.0 (.yaw _relativerotation)) false false)
          (Variables|Default|SetForceUnitVector "0, 0, 0")
          (else
            (Transformation|SetRelativeRotation _arrow_2 (Math|Rotator|MakeRotator (.roll _relativerotation) -84.0 (.yaw _relativerotation)) false false)
            (Variables|Default|SetForceUnitVector "0, 0, 0")))
        (else
          ;;[1 1 1] z축 회전이 범위 안쪽인지 확인
          (Transformation|AddRelativeRotation (Variables|Default|GetArrow) (Math|Rotator|MakeRotator 0.0 (.pitch (Variables|Default|GetForceUnitVector)) 0.0) false false)
          (if (or _returnvalue (< (.yaw _relativerotation_2) -89.0))
            (if _returnvalue
              (Transformation|SetRelativeRotation (Variables|Default|GetArrow) (Math|Rotator|MakeRotator (.roll _relativerotation_3) (.pitch _relativerotation_3) 88.0) false false)
              (Variables|Default|SetForceUnitVector "0, 0, 0")
              (else
                (Transformation|SetRelativeRotation (Variables|Default|GetArrow) (Math|Rotator|MakeRotator (.roll _relativerotation_3) (.pitch _relativerotation_3) -88.0) false false)
                (Variables|Default|SetForceUnitVector "0, 0, 0")))
            (else
              ;[1 1 1] 2
              (if (> (.yaw (Variables|Default|GetForceUnitVector)) 0.0)
                (Development|PrintString (Utilities|String|ToString(Float) (.yaw (Variables|Default|GetForceUnitVector)))))
              (Transformation|AddRelativeRotation (Variables|Default|GetArrow) (Math|Rotator|MakeRotator 0.0 0.0 (.yaw (Variables|Default|GetForceUnitVector))) false false))))))
    (:then_1
      ;;[1 1 1] 엔진컨트롤
      (if (Variables|Default|GetIsEngineOn)
        ;;[1 1 1] 기체 이동
        (Class|PrimitiveComponent|AddForceatLocation (Variables|Default|GetStaticMesh) (* (Math|Vector|GetForwardVector (Variables|Default|GetArrow)) 5e+06) (Transformation|GetWorldLocation (Variables|Default|GetStaticMesh)) "None")))
    (:then_4
      (Variables|Default|SetCurrTime (+ (Variables|Default|GetCurrTime) DeltaSeconds)))))

(fn ConstructionScript)

(fn MakeRotate
  (params (vec :type Vector))
  (return (Math|Rotator|MakeRotator (.z vec) (.y vec) (.x vec))))

(fn CombineRotate
  (params (NewVec :type Vector))
  (bind _forceunitvector (Variables|Default|GetForceUnitVector))
  (bind _rtn (CallFunction|MakeRotate NewVec))
  (return (Math|Rotator|MakeRotator (+ (.roll _forceunitvector) (.roll _rtn)) (+ (.pitch _forceunitvector) (.pitch _rtn)) (+ (.yaw _forceunitvector) (.yaw _rtn)))))