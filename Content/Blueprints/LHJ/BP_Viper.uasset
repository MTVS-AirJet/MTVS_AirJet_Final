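; BP_Viper is a Blueprint that toggles VR headset display mode at runtime from the 9 key.
; A FlipFlop alternates between enabling HMD and stereo with vsync off and raised screen percentage, and reverting to non-stereo with vsync on and a lower resolution.
; Settings are applied mostly through console commands.
; Other rendering tweaks sit in unconnected chains that never run, and BeginPlay and construction are empty.
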(event Collision|EventActorBeginOverlap
  (params (OtherActor :type Actor%20Object%20Reference)))

(event EventTick
  (params (DeltaSeconds :type Float%20%28single-precision%29)))

(event EventBeginPlay)

(event Input|KeyboardEvents|9
  (params (Key :type Key%20Structure :default "None"))
  (:Pressed
    (Utilities|FlowControl|FlipFlop
      (:A
        (Development|ExecuteConsoleCommand "r.vsync 0" 0)
        (Class|HeadMountedDisplayFunctionLibrary|EnableHMD true)
        (Development|ExecuteConsoleCommand "stereo on" 0)
        (Development|ExecuteConsoleCommand "r.setres 1280x720" 0)
        (Development|ExecuteConsoleCommand "sq.ResolutionQuality 100" 0)
        (Development|ExecuteConsoleCommand "r.screenpercentage 150" 0))
      (:B
        (Development|ExecuteConsoleCommand "r.vsync 1" 0)
        (Development|ExecuteConsoleCommand "stereo off" 0)
        (Class|HeadMountedDisplayFunctionLibrary|EnableHMD false)
        (Development|ExecuteConsoleCommand "fullscreen 0" 0)
        (Development|ExecuteConsoleCommand "r.setres 1024x768" 0)
        (Development|ExecuteConsoleCommand "r.HZBOcclusion=0" 0)))))

(fn ConstructionScript)