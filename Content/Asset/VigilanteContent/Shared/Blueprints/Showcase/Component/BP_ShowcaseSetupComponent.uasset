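; BP_ShowcaseSetupComponent is a component that holds the setup data for a showcase on its owning actor.
; Getters expose the showcase name, slot, cameras, separators, and button, checkbox, slider and twin-slider control definitions.
; GetShowcaseControls returns the owner as BP_ShowcaseControlsInterface, printing an error if the actor does not implement it.
; It contains no active event logic, serving purely as a data and lookup provider.
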(event EventBeginPlay)

(event EventTick
  (params (DeltaSeconds :type Float%20%28single-precision%29)))

(fn GetButtonListControls
  (return (Variables|Variables|GetButtonsControls)))

(fn GetCheckboxControls
  (return (Variables|Variables|GetCheckboxControls)))

(fn GetSeparators
  (return (Variables|Variables|GetSeparators)))

(fn GetShowcaseCamera
  (params (Index :type Integer))
  (return (Utilities|Array|Get(acopy) (Variables|Basic|GetShowcaseCameras) Index)))

(fn GetShowcaseCameraCount
  (return (Utilities|Array|Length (Variables|Basic|GetShowcaseCameras))))

(fn GetShowcaseControls
  (bind _returnvalue (Components|GetOwner))
  (if (Utilities|DoesObjectImplementInterface _returnvalue "/Game/Asset/VigilanteContent/Shared/Blueprints/Showcase/Interfaces/BP_ShowcaseControlsInterface.BP_ShowcaseControlsInterface_C")
    (bind _asbp_showcase_controls_interface (Utilities|Casting|CastToBP_ShowcaseControlsInterface (Components|GetOwner)))
    (else
      (Development|PrintString (Utilities|String|Append "Showcase Controls interface not supported in actor: " (Utilities|String|ToString(Object) _returnvalue)))))
  (return _asbp_showcase_controls_interface))

(fn GetShowcaseName
  (return (Variables|Basic|GetName)))

(fn GetShowcaseSlot
  (return (Variables|Basic|GetSlot)))

(fn GetSliderControls
  (return (Variables|Variables|GetSliderControls)))

(fn GetTwinSliderControls
  (return (Variables|Variables|GetTwinSliderControls)))